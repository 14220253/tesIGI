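; Stats component that tracks health and stamina and mirrors them on the player character's HUD.
; On BeginPlay it casts the player character and, after a short delay, fills the widget's bars and health text.
; Functions adjust current and maximum values, capping increases at the maximum; DecreaseHealth returns whether health is depleted.
; DecreaseStamina returns that same health check rather than testing stamina, and its bar update is disconnected.
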(event EventBeginPlay
  (bind _asbp_test_animation_top_down_character (Utilities|Casting|CastToBP_TestAnimationTopDownCharacter (Game|GetPlayerCharacter 0)))
  (Utilities|FlowControl|Delay 0.2)
  (Variables|Default|SetPlayerCharBP _asbp_test_animation_top_down_character)
  (Progress|SetPercent (Variables|/Game/TestAnim/UI/WB_HUD.WB_HUD_C|GetStaminaBar (Variables|/Game/TestAnim/Blueprints/BP_TestAnimationTopDownCharacter.BP_TestAnimationTopDownCharacter_C|GetHUDWidget (Variables|Default|GetPlayerCharBP))) (/ (Variables|Stamina|GetCurrentStamina) (Variables|Stamina|GetMaxStamina)))
  (Progress|SetPercent (Variables|/Game/TestAnim/UI/WB_HUD.WB_HUD_C|GetHealthBar (Variables|/Game/TestAnim/Blueprints/BP_TestAnimationTopDownCharacter.BP_TestAnimationTopDownCharacter_C|GetHUDWidget (Variables|Default|GetPlayerCharBP))) (/ (Variables|Health|GetCurrentHealth) (Variables|Health|GetMaxHealth)))
  (Rendering|Components|TextRender|SetText (Variables|/Game/TestAnim/UI/WB_HUD.WB_HUD_C|GetHealthText (Variables|/Game/TestAnim/Blueprints/BP_TestAnimationTopDownCharacter.BP_TestAnimationTopDownCharacter_C|GetHUDWidget (Variables|Default|GetPlayerCharBP))) (Utilities|Text|ToText(Float) (Variables|Health|GetCurrentHealth) "HalfToEven")))

(fn DecreaseHealth
  (params (Damage :type Float%20%28double-precision%29))
  (bind _playercharbp (Variables|Default|GetPlayerCharBP))
  (bind _hudwidget (Variables|/Game/TestAnim/Blueprints/BP_TestAnimationTopDownCharacter.BP_TestAnimationTopDownCharacter_C|GetHUDWidget _playercharbp))
  (bind _output_get (Variables|Health|SetCurrentHealth (- (Variables|Health|GetCurrentHealth) Damage)))
  (Progress|SetPercent (Variables|/Game/TestAnim/UI/WB_HUD.WB_HUD_C|GetHealthBar _hudwidget) (/ _output_get (Variables|Health|GetMaxHealth)))
  (Rendering|Components|TextRender|SetText (Variables|/Game/TestAnim/UI/WB_HUD.WB_HUD_C|GetHealthText _hudwidget) (Utilities|Text|ToText(Float) (Variables|Health|GetCurrentHealth) "HalfToEven"))
  (if (<= (Variables|Health|GetCurrentHealth) 0.0)
    (return true)
    (else
      (return false))))

(fn IncreaseMaxHealth
  (params (IncrementHealth :type Float%20%28double-precision%29))
  (bind _playercharbp (Variables|Default|GetPlayerCharBP))
  (bind _hudwidget (Variables|/Game/TestAnim/Blueprints/BP_TestAnimationTopDownCharacter.BP_TestAnimationTopDownCharacter_C|GetHUDWidget _playercharbp))
  (Variables|Health|SetMaxHealth (+ (Variables|Health|GetMaxHealth) IncrementHealth))
  (Progress|SetPercent (Variables|/Game/TestAnim/UI/WB_HUD.WB_HUD_C|GetHealthBar _hudwidget) (/ (Variables|Health|GetCurrentHealth) (Variables|Health|GetMaxHealth)))
  (Rendering|Components|TextRender|SetText (Variables|/Game/TestAnim/UI/WB_HUD.WB_HUD_C|GetHealthText _hudwidget) (Utilities|Text|ToText(Float) (Variables|Health|GetCurrentHealth) "HalfToEven")))

(fn DecreaseStamina
  (params (StaminaDepleted :type Float%20%28double-precision%29))
  (Variables|Stamina|SetCurrentStamina (- (Variables|Stamina|GetCurrentStamina) StaminaDepleted))
  (if (<= (Variables|Health|GetCurrentHealth) 0.0)
    (return true)
    (else
      (return false))))

(fn IncreaseMaxStamina
  (params (AddedStamina :type Float%20%28double-precision%29))
  (Variables|Stamina|SetMaxStamina (+ (Variables|Stamina|GetMaxStamina) AddedStamina))
  (Progress|SetPercent (Variables|/Game/TestAnim/UI/WB_HUD.WB_HUD_C|GetStaminaBar (Variables|/Game/TestAnim/Blueprints/BP_TestAnimationTopDownCharacter.BP_TestAnimationTopDownCharacter_C|GetHUDWidget (Variables|Default|GetPlayerCharBP))) (/ (Variables|Stamina|GetCurrentStamina) (Variables|Stamina|GetMaxStamina))))

(fn IncreaseHealth
  (params (AddedHealth :type Float%20%28double-precision%29))
  (bind _playercharbp (Variables|Default|GetPlayerCharBP))
  (bind _hudwidget (Variables|/Game/TestAnim/Blueprints/BP_TestAnimationTopDownCharacter.BP_TestAnimationTopDownCharacter_C|GetHUDWidget _playercharbp))
  (Variables|Health|SetCurrentHealth (+ (Variables|Health|GetCurrentHealth) AddedHealth))
  (if (> (Variables|Health|GetCurrentHealth) (Variables|Health|GetMaxHealth))
    (Variables|Health|SetCurrentHealth (Variables|Health|GetMaxHealth)))
  (Progress|SetPercent (Variables|/Game/TestAnim/UI/WB_HUD.WB_HUD_C|GetHealthBar _hudwidget) (/ (Variables|Health|GetCurrentHealth) (Variables|Health|GetMaxHealth)))
  (Rendering|Components|TextRender|SetText (Variables|/Game/TestAnim/UI/WB_HUD.WB_HUD_C|GetHealthText _hudwidget) (Utilities|Text|ToText(Float) (Variables|Health|GetCurrentHealth) "HalfToEven")))

(fn IncreaseStamina
  (params (Added%20Stamina :type Float%20%28double-precision%29))
  (Variables|Stamina|SetCurrentStamina (+ (Variables|Stamina|GetCurrentStamina) Added%20Stamina))
  (if (> (Variables|Stamina|GetCurrentStamina) (Variables|Stamina|GetMaxStamina))
    (Variables|Stamina|SetCurrentStamina (Variables|Stamina|GetMaxStamina)))
  (Progress|SetPercent (Variables|/Game/TestAnim/UI/WB_HUD.WB_HUD_C|GetStaminaBar (Variables|/Game/TestAnim/Blueprints/BP_TestAnimationTopDownCharacter.BP_TestAnimationTopDownCharacter_C|GetHUDWidget (Variables|Default|GetPlayerCharBP))) (/ (Variables|Stamina|GetCurrentStamina) (Variables|Stamina|GetMaxStamina))))